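; BP_RapaPawn is a sample pawn that moves and turns from player axis input.
; MoveForward offsets the root scene component along the actor's forward vector, while MoveRight sets a new location along the right vector, both with sweep enabled.
; Turn adds the axis value to the actor's yaw, keeping pitch and roll.
; All three apply raw axis values directly, without delta-time scaling or a movement component.
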(event `self.ReceiveBeginPlay`)

(event `InputAxis|MoveForward`
  (params (AxisValue :type "Float (single-precision)"))
  (`SceneComponent.K2_AddWorldOffset` (`self.DefaultSceneRoot`) (* (`KismetMathLibrary.GetForwardVector` (`self.K2_GetActorRotation`)) AxisValue) true false))

(event `InputAxis|MoveRight`
  (params (AxisValue :type "Float (single-precision)"))
  (`self.K2_SetActorLocation` (+ (* (`KismetMathLibrary.GetRightVector` (`self.K2_GetActorRotation`)) AxisValue) (`self.K2_GetActorLocation`)) true))

(event `InputAxis|Turn`
  (params (AxisValue :type "Float (single-precision)"))
  (bind (_returnvalue_roll _returnvalue_pitch _returnvalue_yaw) (`KismetMathLibrary.BreakRotator` (`self.K2_GetActorRotation`)))
  (bind (_returnvalue_roll_2 _returnvalue_pitch_2 _returnvalue_yaw_2) (`KismetMathLibrary.BreakRotator` (`KismetMathLibrary.MakeRotator` 0.0 0.0 (* AxisValue 1.0))))
  (`self.K2_SetActorRotation` (`KismetMathLibrary.MakeRotator` _returnvalue_roll _returnvalue_pitch (+ _returnvalue_yaw _returnvalue_yaw_2))))

(fn `UserConstructionScript`)